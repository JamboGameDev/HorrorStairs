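; BP_Hints is a trigger-volume actor that shows the player an on-screen control hint, such as the flashlight or interaction key.
; On BeginPlay it creates a WP_Hint widget and sets its text from the HintType enum.
; Box overlap events cast to HP_Character, adding the widget to the viewport on entry and removing it on exit.
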(event OnComponentBeginOverlap(Box)
  (params (OverlappedComponent :type Primitive%20Component%20Object%20Reference) (OtherActor :type Actor%20Object%20Reference) (OtherComp :type Primitive%20Component%20Object%20Reference) (OtherBodyIndex :type Integer) (bFromSweep :type Boolean) (SweepResult :type Hit%20Result%20Structure%20%28by%20ref%29))
  (Utilities|Casting|CastToHP_Character OtherActor)
  (UserInterface|Viewport|AddtoViewport (Variables|Default|GetHintRef) 0))

(event OnComponentEndOverlap(Box)
  (params (OverlappedComponent :type Primitive%20Component%20Object%20Reference) (OtherActor :type Actor%20Object%20Reference) (OtherComp :type Primitive%20Component%20Object%20Reference) (OtherBodyIndex :type Integer))
  (Utilities|Casting|CastToHP_Character OtherActor)
  (Widget|RemovefromParent (Variables|Default|GetHintRef)))

(event EventBeginPlay
  (bind _returnvalue (UserInterface|CreateWidget "/Game/Wigets/WP_Hint.WP_Hint_C"))
  (bind _output_get (Variables|Default|SetHintRef _returnvalue))
  (switch Utilities|FlowControl|Switch|SwitchonE_Hints (Variables|Default|GetHintType)
    (:NewEnumerator0
      (Variables|/Game/Wigets/WP_Hint.WP_Hint_C|SetHintTextVar _output_get "F for flashlight"))
    (:NewEnumerator1
      (Variables|/Game/Wigets/WP_Hint.WP_Hint_C|SetHintTextVar _output_get "E for interaction"))))

(event Collision|EventActorBeginOverlap
  (params (OtherActor :type Actor%20Object%20Reference)))

(event EventTick
  (params (DeltaSeconds :type Float%20%28single-precision%29)))

(fn ConstructionScript)