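; Trigger-box actor that fires a one-time jumpscare when the HP_Character enters it.
; A DoOnce gate feeds a switch on JumpscareType, so one Blueprint covers every scare variant.
; Variants show a timed fake Windows error widget with cursor, play 2D stingers, or drop staggered BP_Can actors around CubeSpawn.
; Others act on the overlapping character, toggling or breaking its flashlight or turning on madness.
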(event OnComponentBeginOverlap(Box)
  (params (OverlappedComponent :type Primitive%20Component%20Object%20Reference) (OtherActor :type Actor%20Object%20Reference) (OtherComp :type Primitive%20Component%20Object%20Reference) (OtherBodyIndex :type Integer) (bFromSweep :type Boolean) (SweepResult :type Hit%20Result%20Structure%20%28by%20ref%29))
  (bind _cubespawn (Variables|Default|GetCubeSpawn))
  (bind _cubespawn_2 (Variables|Default|GetCubeSpawn))
  (bind _cubespawn_3 (Variables|Default|GetCubeSpawn))
  (bind _returnvalue (Transformation|GetWorldLocation _cubespawn_2))
  (bind _returnvalue_2 (Transformation|GetWorldLocation _cubespawn_3))
  (bind _returnvalue_3 (Transformation|GetWorldLocation _cubespawn))
  (bind _ashp_character (Utilities|Casting|CastToHP_Character OtherActor))
  (Utilities|FlowControl|DoOnce false
    (:Completed
      (switch Utilities|FlowControl|Switch|SwitchonE_JumpscareType (Variables|Default|GetJumpscareType)
        (:NewEnumerator0
          (bind _returnvalue_4 (UserInterface|CreateWidget "/Game/Wigets/WB_Jumpscare.WB_Jumpscare_C"))
          (UserInterface|Viewport|AddtoViewport _returnvalue_4 0)
          (Audio|PlaySound2D "/Game/Content/Sounds/WindowsScare_8_The_Windows_Error_by_s0m3us3r12346877_Id_624667.WindowsScare_8_The_Windows_Error_by_s0m3us3r12346877_Id_624667" 1.0 1.0 0.0 0 0)
          (Variables|/Script/Engine.PlayerController|SetbShowMouseCursor (Game|GetPlayerController 0) true)
          (Utilities|FlowControl|Delay 3.0)
          (Widget|RemovefromParent _returnvalue_4)
          (Variables|/Script/Engine.PlayerController|SetbShowMouseCursor (Game|GetPlayerController 0) false))
        (:NewEnumerator1
          (Audio|PlaySound2D "/Game/Content/Sounds/JumpScare_33-Jumpscare_Sfx__3__by_dragonboi50120_Id-631976.JumpScare_33-Jumpscare_Sfx__3__by_dragonboi50120_Id-631976" 1.0 1.0 0.0 0 0))
        (:NewEnumerator2
          (Audio|PlaySound2D "/Game/Content/Sounds/JumpScare_35-Jumpscare_by_TheLastEmber_Id-795247.JumpScare_35-Jumpscare_by_TheLastEmber_Id-795247" 1.0 1.0 0.0 0 0))
        (:NewEnumerator3
          (Game|SpawnActorfromClass "/Game/BP/BP_Can.BP_Can_C" (Math|Transform|MakeTransform (Math|Vector|MakeVector (+ (.x _returnvalue) 1e+02) (.y _returnvalue) (.z _returnvalue)) "0, 0, 0" "1.000000,1.000000,1.000000") "Undefined" "MultiplyWithRoot" 0 0)
          (Utilities|FlowControl|Delay 0.2)
          (Game|SpawnActorfromClass "/Game/BP/BP_Can.BP_Can_C" (Math|Transform|MakeTransform (Math|Vector|MakeVector (.x _returnvalue_2) (+ (.y _returnvalue_2) 2e+02) (.z _returnvalue_2)) "0, 0, 0" "1.000000,1.000000,1.000000") "Undefined" "MultiplyWithRoot" 0 0)
          (Utilities|FlowControl|Delay 0.3)
          (Game|SpawnActorfromClass "/Game/BP/BP_Can.BP_Can_C" (Math|Transform|MakeTransform (Math|Vector|MakeVector (+ (.x _returnvalue_3) -1.3e+02) (+ (.y _returnvalue_3) -1.5e+02) (.z _returnvalue_3)) "0, 0, 0" "1.000000,1.000000,1.000000") "Undefined" "MultiplyWithRoot" 0 0))
        (:NewEnumerator4
          (Default|ChangeFlashlight _ashp_character))
        (:NewEnumerator5
          (Default|BrokeFlashlight6 _ashp_character))
        (:NewEnumerator6
          (Default|BroKeFlashlight7 _ashp_character))
        (:NewEnumerator7
          (Variables|/Game/BP/HP_Character.HP_Character_C|SetMadnessOn? _ashp_character true)
          (Audio|PlaySound2D "/Game/Content/Sounds/JumpScare_36-Echo_Jumpscare_by_Sapisvr_Id-371709.JumpScare_36-Echo_Jumpscare_by_Sapisvr_Id-371709" 1.0 1.0 0.0 0 0))))))

(event EventBeginPlay)

(event Collision|EventActorBeginOverlap
  (params (OtherActor :type Actor%20Object%20Reference)))

(event EventTick
  (params (DeltaSeconds :type Float%20%28single-precision%29)))

(fn ConstructionScript)